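; Elevator actor that moves between relative locations using an InterpToMovement component.
; The construction script builds a path from Location1 to Location2 and applies the Duration.
; Any actor overlap sets OnElevator, which is never cleared and lets the EventFloor1 event replace the control points with Location2 and reapply Duration.
; It appears unfinished: debug prints remain, Location3 and Location4 nodes are unused, and a Delay is disconnected.
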(event `self.ReceiveActorBeginOverlap`
  (params (OtherActor :type "Actor Object Reference"))
  (`KismetSystemLibrary.PrintString` "Hello")
  (set `self.OnElevator` true))

(event `Key|One`
  (params (Key :type "Key Structure")))

(event `EventFloor1`
  (bind _interptomovement (`self.InterpToMovement`))
  (if (`self.OnElevator`)
    (`KismetSystemLibrary.PrintString` "Move")
    (set `InterpToMovementComponent.ControlPoints` (`|MakeArray` (make `InterpControlPoint` (`self.Location2`)) (struct) (struct) (struct)) _interptomovement)
    (set `InterpToMovementComponent.Duration` (`self.Duration`) _interptomovement)))

(fn `UserConstructionScript`
  (bind _interptomovement (`self.InterpToMovement`))
  (set `InterpToMovementComponent.ControlPoints` (`|MakeArray` (make `InterpControlPoint` (`self.Location1`)) (make `InterpControlPoint` (`self.Location2`)) (struct) (struct) (struct)) _interptomovement)
  (set `InterpToMovementComponent.Duration` (`self.Duration`) _interptomovement))