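; Enemy pawn that chases the player character on sight and can be damaged and destroyed.
; PawnSensing triggers AI MoveTo toward the seen character, while one sphere's overlaps show and hide the health widget for the player.
; A second sphere's overlap with any actor opens a half-second hit window.
; HealthDrop subtracts health only inside that window, destroying the enemy and playing a sound at zero.
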(event `self.ReceiveBeginPlay`
  (bind _asenemy_health (cast `/Game/ThirdPersonBP/Blueprints/TPIGA/EnemyHealth` (`WidgetComponent.GetUserWidgetObject` (`self.EnemyHealthWidget`))))
  (set `self.HealthWidgetRef` _asenemy_health))

(event `self.PawnSensing.OnSeePawn`
  (params (Pawn :type "Pawn Object Reference"))
  (bind _asthird_person_character (cast `/Game/ThirdPersonBP/Blueprints/ThirdPersonCharacter` Pawn))
  (`|AIMoveTo` self (0.0 0.0 0.0) _asthird_person_character))

(event `self.EnemySphereH.OnComponentBeginOverlap`
  (params (OverlappedComponent :type "PrimitiveComponent Object Reference") (OtherActor :type "Actor Object Reference") (OtherComp :type "PrimitiveComponent Object Reference") (OtherBodyIndex :type Integer) (bFromSweep :type Boolean) (SweepResult :type "HitResult Structure (by ref)"))
  ;[1 1 1] Makes Enemy Health Appear and Dissapear
  (cast `/Game/ThirdPersonBP/Blueprints/ThirdPersonCharacter` OtherActor)
  (`SceneComponent.SetVisibility` (`self.EnemyHealthWidget`) true false))

(event `self.EnemySphereH.OnComponentEndOverlap`
  (params (OverlappedComponent :type "PrimitiveComponent Object Reference") (OtherActor :type "Actor Object Reference") (OtherComp :type "PrimitiveComponent Object Reference") (OtherBodyIndex :type Integer))
  ;[1 1 1] Makes Enemy Health Appear and Dissapear
  (cast `/Game/ThirdPersonBP/Blueprints/ThirdPersonCharacter` OtherActor)
  (`SceneComponent.SetVisibility` (`self.EnemyHealthWidget`) false false))

(event `HealthDrop`
  ;[1 1 1] Lowers Enemy1's Health
  (`KismetSystemLibrary.PrintString` "Before Damage")
  (if (`self.PlayerWithinRange`)
    (set `self.Health` (- (`self.Health`) 10.0))
    (`KismetSystemLibrary.PrintString` "DAMAGE Dealt")
    (if (<= (`self.Health`) 0.0)
      (`self.K2_DestroyActor`)
      (`GameplayStatics.PlaySoundAtLocation` "/Game/ThirdPersonBP/Blueprints/Audio/Disappearing_yellow_emoji_meme__getmp3_pro_.Disappearing_yellow_emoji_meme__getmp3_pro_" (`self.K2_GetActorLocation`) (struct) 1.0 1.0 0.0 null null null))))

(event `self.EnemySphereHit.OnComponentBeginOverlap`
  (params (OverlappedComponent :type "PrimitiveComponent Object Reference") (OtherActor :type "Actor Object Reference") (OtherComp :type "PrimitiveComponent Object Reference") (OtherBodyIndex :type Integer) (bFromSweep :type Boolean) (SweepResult :type "HitResult Structure (by ref)"))
  ;[1 1 1] Finds out if player is within range to strike Enemy1
  (set `self.PlayerWithinRange` true)
  (`KismetSystemLibrary.Delay` 0.5)
  (set `self.PlayerWithinRange` false))

(event `self.EnemySphereHit.OnComponentEndOverlap`
  (params (OverlappedComponent :type "PrimitiveComponent Object Reference") (OtherActor :type "Actor Object Reference") (OtherComp :type "PrimitiveComponent Object Reference") (OtherBodyIndex :type Integer))
  ;[1 1 1] Finds out if player is within range to strike Enemy1
)

(fn `UserConstructionScript`)